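; Gameplay ability for the Mountain Dragon boss's wipe attack, which players survive by gaining height.
; The dragon moves to its wipe point, faces the nearest player and plays a wake-up montage while a blackboard flag marks the cast.
; A downward trace places grid-snapped safety stairs ahead and starts a floor warning, then a delayed shout triggers the height-based kill.
; If the trace misses, it only spawns fallback stairs and never ends the ability.
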(event Ability|EventActivateAbilityFromEvent
  (params (EventData :type Gameplay%20Event%20Data%20Structure%20%28by%20ref%29))
  (bind _returnvalue (Ability|GetAvatarActorfromActorInfo))
  (bind _returnvalue_2 (AI|GetAIController _returnvalue))
  (AI|Navigation|StopMovement _returnvalue_2)
  (bind _asbp_boss_dragon (Utilities|Casting|CastToBP_BossDragon _returnvalue))
  (AI|Components|Blackboard|SetValueasBool (AI|GetBlackboard (AI|GetAIController _asbp_boss_dragon)) (Utilities|Name|MakeLiteralName "IsCastingWipe") true)
  (AI|AIMoveTo _asbp_boss_dragon (Transformation|GetActorLocation (Variables|/Script/Enemy.BossDragon|GetWipeTargetPoint _asbp_boss_dragon)) 0 5.0 false
    (:OnSuccess
      (bind _asdragon_ai (Utilities|Casting|CastToDragonAI _returnvalue_2))
      (bind _returnvalue_3 (Class|DragonAI|UpdateTargettoNearestPlayer _asdragon_ai))
      (Default|RotatetoTarget _asbp_boss_dragon _returnvalue_3)
      (Utilities|FlowControl|Delay 0.8)
      (|PlayMontageandWaitProxy "None" "/Game/Enemy/Boss/MountainDragon/Animations/Dragon_WakeUp.Dragon_WakeUp" 1.0 "None" true 1.0 0.0 false
        (:OnCompleted
          (bind (_outhit _returnvalue_4) (Collision|LineTraceByChannel (+ (+ (Transformation|GetActorLocation _asbp_boss_dragon) (* (Transformation|GetActorForwardVector _asbp_boss_dragon) 1e+03)) "0.000000,0.000000,500.000000") (- (+ (Transformation|GetActorLocation _asbp_boss_dragon) (* (Transformation|GetActorForwardVector _asbp_boss_dragon) 1e+03)) "0.000000,0.000000,1000.000000") "TraceTypeQuery1" false 0 "ForDuration"))
          (if _returnvalue_4
            (Class|BossDragon|SpawnSafetyStairs _asbp_boss_dragon (Math|Vector|MakeVector (Math|Float|SnapToGrid(Float) (.x (.impactpoint _outhit)) 1e+02) (Math|Float|SnapToGrid(Float) (.y (.impactpoint _outhit)) 1e+02) (+ (.z (.impactpoint _outhit)) 5e+01)) 3 1e+01)
            (Class|BossDragon|SetFloorWarningState _asbp_boss_dragon (Transformation|GetActorLocation _asbp_boss_dragon) 1.8e+03 true)
            (Utilities|FlowControl|Delay 5.0)
            (|PlayMontageandWaitProxy "None" "/Game/Enemy/Boss/MountainDragon/Animations/Dragon_Shout.Dragon_Shout" 0.8 "None" true 1.0 0.0 false
              (:OnCompleted
                (Class|BossDragon|ExecuteHeightJudgmentKill _asbp_boss_dragon 2.5e+02)
                (Class|BossDragon|SetFloorWarningState _asbp_boss_dragon (Transformation|GetActorLocation _asbp_boss_dragon) 1.8e+03 false)
                (AI|Components|Blackboard|SetValueasBool (AI|GetBlackboard (AI|GetAIController _asbp_boss_dragon)) (Utilities|Name|MakeLiteralName "IsCastingWipe") false)
                (Ability|EndAbility)))
            (else
              (Class|BossDragon|SpawnSafetyStairs _asbp_boss_dragon (+ (Transformation|GetActorLocation _asbp_boss_dragon) (* (Transformation|GetActorForwardVector _asbp_boss_dragon) 1e+03)) 0 15.0))))))))