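; Gameplay ability that makes the Mountain Dragon boss perform a straight-line rush toward its target.
; It raises movement speed and acceleration, then uses AI MoveTo toward a point a set charge distance along the direction to the blackboard's TargetActor.
; The rush montage plays alongside the move, and only its completion restores normal movement and ends the ability.
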(event Ability|EventActivateAbility
  (bind _asbp_boss_dragon (Utilities|Casting|CastToBP_BossDragon (Ability|GetAvatarActorfromActorInfo)))
  (Variables|/Script/Engine.CharacterMovementComponent|SetMaxWalkSpeed (Variables|/Script/Engine.Character|GetCharacterMovement _asbp_boss_dragon) (Variables|Default|GetRushSpeed))
  (Variables|/Script/Engine.CharacterMovementComponent|SetMaxAcceleration (Variables|/Script/Engine.Character|GetCharacterMovement _asbp_boss_dragon) (Variables|Default|GetRushAccel))
  (bind _as캐릭터 (Utilities|Casting|CastToCharacter (AI|Components|Blackboard|GetValueasObject (AI|GetBlackboard (Pawn|GetController _asbp_boss_dragon)) (Utilities|Name|MakeLiteralName "TargetActor"))))
  (AI|AIMoveTo _asbp_boss_dragon (+ (* (Math|Vector|GetUnitDirection(Vector) (Transformation|GetActorLocation _asbp_boss_dragon) (Transformation|GetActorLocation _as캐릭터)) (Variables|Default|GetChargeDistance)) (Transformation|GetActorLocation _asbp_boss_dragon)) 0 5.0 false
    (:then
      (|PlayMontageandWaitProxy "None" (Variables|Default|GetRushMontage) 1.0 "None" true 1.0 0.0 false
        (:OnCompleted
          (Variables|/Script/Engine.CharacterMovementComponent|SetMaxWalkSpeed (Variables|/Script/Engine.Character|GetCharacterMovement _asbp_boss_dragon) (Variables|Default|GetNormalSpeed))
          (Variables|/Script/Engine.CharacterMovementComponent|SetMaxAcceleration (Variables|/Script/Engine.Character|GetCharacterMovement _asbp_boss_dragon) (Variables|Default|GetNormalAccel))
          (Ability|EndAbility))))))