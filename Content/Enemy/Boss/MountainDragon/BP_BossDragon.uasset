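; BP_BossDragon is the Mountain Dragon boss enemy, providing events for turning toward a target and displaying damage taken.
; RotateToTarget plays the walk montage while a timeline interpolates from the current rotation to a yaw-only look-at rotation, keeping the dragon upright.
; ShowDamageNumber spawns a BP_DamageActor at the dragon's location, passing it the damage amount.
; The file holds no other behavior, as BeginPlay and the construction script are empty.
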(event Custom|RotateToTarget
  (params (TargetActor :type Actor%20Object%20Reference))
  (Variables|Default|SetStartRot (Transformation|GetActorRotation))
  (Variables|Default|SetTargetRot (Math|Rotator|MakeRotator 0.0 0.0 (.Yaw (Math|Rotator|BreakRotator (Math|Rotator|FindLookatRotation (Transformation|GetActorLocation) (Transformation|GetActorLocation TargetActor))))))
  (Animation|PlayAnimMontage "/Game/Enemy/Boss/MountainDragon/Animations/Dragon_Walk.Dragon_Walk" 1.0 "None")
  (bind _회전 (Timeline|Rotation PlayFromStart)
    (:Update
      (Transformation|SetActorRotation (Math|Rotator|Lerp(Rotator) (Variables|Default|GetStartRot) (Variables|Default|GetTargetRot) _회전)))))

(event EventBeginPlay)

(event EventShowDamageNumber
  (params (DamageAmount :type Float%20%28single-precision%29))
  (Game|SpawnActorfromClass "/Game/UI/BP_DamageActor.BP_DamageActor_C" (Math|Conversions|ToTransform(Vector) (Transformation|GetActorLocation)) "AlwaysSpawn" "MultiplyWithRoot" 0 DamageAmount 0))

(fn ConstructionScript)